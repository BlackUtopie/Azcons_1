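; BP_BaseInteract is a base interactable object that announces itself to the player character by proximity.
; Begin and end overlaps on TriggerInteract cast the other actor to ThirdPersonCharacter, then register or unregister this object through interactable message calls.
; The construction script applies MeshScale to the SMItem mesh.
; SetOutline always disables custom depth rendering on that mesh, ignoring its Outlight input.
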(event OnComponentBeginOverlap(TriggerInteract)
  (params (OverlappedComponent :type Primitive%20Component%20Object%20Reference) (OtherActor :type Actor%20Object%20Reference) (OtherComp :type Primitive%20Component%20Object%20Reference) (OtherBodyIndex :type Integer) (bFromSweep :type Boolean) (SweepResult :type Hit%20Result%20Structure%20%28by%20ref%29))
  (bind _asthird_person_character (Utilities|Casting|CastToThirdPersonCharacter OtherActor))
  (Class|BPIInteract|RegisterInteractable(Message) _asthird_person_character self))

(event OnComponentEndOverlap(TriggerInteract)
  (params (OverlappedComponent :type Primitive%20Component%20Object%20Reference) (OtherActor :type Actor%20Object%20Reference) (OtherComp :type Primitive%20Component%20Object%20Reference) (OtherBodyIndex :type Integer))
  (bind _asthird_person_character (Utilities|Casting|CastToThirdPersonCharacter OtherActor))
  (Class|BPIInteract|UnregisterInteractable(Message) _asthird_person_character self))

(fn ConstructionScript
  (Transformation|SetWorldScale3D (Variables|Default|GetSM_Item) (Variables|Size|GetMesh_Scale)))

(fn SetOutline
  (params (Outlight? :type Boolean))
  (Rendering|SetRenderCustomDepth (Variables|Default|GetSM_Item) false))