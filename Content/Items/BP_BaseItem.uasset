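; Base pickup item actor that a character can collect into an inventory through an Interactable event.
; On interaction it checks that the character has inventory space, passes its ItemInfo to the character's PickUpMessage, then destroys itself.
; The construction script rebuilds ItemInfo with the actor's own class filled in, keeping the other fields, so the passed data identifies which item class it came from.
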(event EventInteractable
  (params (Character :type Third%20Person%20Character%20Object%20Reference))
  (if (Default|HasSpaceInventory Character)
    (Class|BPIInteract|PickUp(Message) Character (Variables|Default|GetItemInfo))
    (Actor|DestroyActor)))

(fn ConstructionScript
  (|CallParentFunction)
  (Variables|Default|SetItemInfo (Utilities|Struct|MakeS_ItemInfo (.itemtype (Variables|Default|GetItemInfo)) (.itemname (Variables|Default|GetItemInfo)) (.itemdescription (Variables|Default|GetItemInfo)) (.itemicon (Variables|Default|GetItemInfo)) (Utilities|GetClass self) (.itemindex (Variables|Default|GetItemInfo)))))